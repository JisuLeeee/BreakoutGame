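; B_Ball is the Breakout ball, moving in the YZ plane from a random start direction while the game runs unpaused.
; Tick moves it with a swept SetActorLocation, and hits reflect its direction about the surface normal.
; Hits notify GI_BreakOut and play sounds; Ground destroys the ball, reporting game over if flagged as main.
; Functions expose clamped speed changes and a timed damage boost.
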(event OnComponentHit(SM_Ball)
  (params (HitComponent :type Primitive%20Component%20Object%20Reference) (OtherActor :type Actor%20Object%20Reference) (OtherComp :type Primitive%20Component%20Object%20Reference) (NormalImpulse :type Vector :default "0, 0, 0") (Hit :type Hit%20Result%20Structure%20%28by%20ref%29))
  ;[1 1 1] 공이 충돌할 때 나아가는 방향 변경
  (bind _newdirection (Ball|ChangeDirection Hit (Variables|Ball|GetDirection)))
  (Variables|Ball|SetDirection _newdirection)
  (Utilities|FlowControl|Sequence
    (:then_0
      ;[1 1 1] 공이 벽과 부딪혔을 때 Combo 및 TriggerCount 변수 세팅
      (if (Actor|ActorHasTag OtherActor "Wall")
        (Default|OnWallHitReset (Variables|Ball|GetGI_BreakOut))
        (Audio|PlaySound2D "/Game/Sounds/A_WallHit.A_WallHit" 1.0 1.0 0.0 0 0)
        (else
          (Utilities|Casting|CastToB_Brick OtherActor
            (:then
              (Default|OnBrickHit (Variables|Ball|GetGI_BreakOut))
              (Audio|PlaySound2D "/Game/Sounds/A_BrickHit.A_BrickHit" 1.0 1.0 0.0 0 0))
            (:CastFailed
              (Default|OnNonBrickContact (Variables|Ball|GetGI_BreakOut)))))))
    (:then_1
      ;[1 1 1] 공이 바닥과 부딪혔을 때 메인공 및 서브공 파괴 & [패배조건①] 메인공이 바닥에 닿으면 LoseWidget으로 이동
      (if (Actor|ActorHasTag OtherActor "Ground")
        (Utilities|FlowControl|Sequence
          (:then_0
            (Actor|DestroyActor))
          (:then_1
            (if (Variables|Ball|GetbCausesGameOver)
              (Default|OnMainBallOut (Variables|Ball|GetGI_BreakOut)))))))
    (:then_2
      (Utilities|Casting|CastToB_Player OtherActor)
      (Audio|PlaySound2D "/Game/Sounds/PaddleHit.PaddleHit" 1.0 1.0 0.0 0 0))))

(event EventBeginPlay
  (bind _asgi_break_out (Utilities|Casting|CastToGI_BreakOut (Game|GetGameInstance)))
  (Variables|Ball|SetGI_BreakOut _asgi_break_out)
  (Variables|Ball|SetDirection (Math|Vector|Normalize (Math|Vector|MakeVector 0.0 (Math|Random|RandomFloatinRange 0.5 1.0) (Math|Random|RandomFloatinRange 0.5 1.0)))))

(event Collision|EventActorBeginOverlap
  (params (OtherActor :type Actor%20Object%20Reference)))

(event EventTick
  (params (DeltaSeconds :type Float%20%28single-precision%29))
  (bind _gi_breakout (Variables|Ball|GetGI_BreakOut))
  ;[1 1 1] 게임이 진행 상태일 때
  (if (and (Default|GetIsRunning _gi_breakout) (not (Default|GetIsPaused _gi_breakout)))
    ;[1 1 1] 공의 위치 업데이트 [New Location = Current Location + ((Direction*Speed)*DeltaTime)]
    (Transformation|SetActorLocation (+ (* DeltaSeconds (* (Variables|Ball|GetDirection) (Variables|Ball|GetSpeed))) (Transformation|GetActorLocation)) true false)))

(fn ConstructionScript)

(fn GetSpeed
  (return (Variables|Ball|GetSpeed)))

(fn SetSpeed
  (params (InSpeed :type Float%20%28double-precision%29))
  (Variables|Ball|SetSpeed (Math|Float|Clamp(Float) InSpeed 3.5e+02 8e+02))
  (return))

(fn SpeedUp
  (Variables|Ball|SetSpeed (Math|Float|Clamp(Float) (+ (Variables|Ball|GetSpeed) 1e+02) 3.5e+02 8e+02))
  (return))

(fn SpeedDown
  (Variables|Ball|SetSpeed (Math|Float|Clamp(Float) (- (Variables|Ball|GetSpeed) 1e+02) 3.5e+02 8e+02))
  (return))

(fn GetDamage
  (return (Variables|Ball|GetDamage)))

(fn IncreaseDamage
  (bind _output_get (Variables|Ball|SetDamage (Math|Integer|Clamp(Integer) 2 1 2)))
  (if (== _output_get 2)
    (Utilities|Time|ClearandInvalidateTimerbyHandle (Variables|Ball|GetResetTimer))
    (Utilities|Time|SetTimerbyFunctionName 0 "ResetDamage" 1e+01) ; 공의 데미지 증가 시간 설정
    (return)))

(fn ResetDamage
  (Variables|Ball|SetDamage 1)
  (return))

(fn GetLocation
  (return (Transformation|GetWorldLocation (Variables|Default|GetSM_Ball))))

(fn GetDirection
  (return (Variables|Ball|GetDirection)))

(fn SetDirection
  (params (Direction :type Vector))
  (Variables|Ball|SetDirection Direction)
  (return))

(fn ChangeDirection
  (params (Hit :type Hit%20Result%20Structure%20%28by%20ref%29) (InDirection :type Vector))
  (bind _normal (Collision|BreakHitResult Hit))
  (bind _returnvalue (Math|Vector|DotProduct _normal InDirection))
  (bind _returnvalue_2 (* _normal _returnvalue))
  (bind _returnvalue_3 (* _returnvalue_2 2.0))
  (bind _returnvalue_4 (- InDirection _returnvalue_3))
  (bind (_x _y _z) (Math|Vector|BreakVector _returnvalue_4))
  (return (Math|Vector|MakeVector 0.0 _y _z)))

(fn SetCausesGameOver
  (params (bCausesGameOver :type Boolean))
  (Variables|Ball|SetbCausesGameOver bCausesGameOver)
  (return))