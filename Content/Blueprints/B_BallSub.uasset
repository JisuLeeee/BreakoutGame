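; Secondary ball for a brick-breaker game, a child of a ball Blueprint that does not cause game over.
; It starts with its own HP and damage, losing HP on each brick hit.
; At zero HP it waits a zero-length Delay before destroying itself so the last hit still damages the brick.
; GetDamage returns its own damage, while empty overrides disable inherited speed changes, damage increases and overlap handling.
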(event OnComponentHit(SM_Ball)
  (params (HitComponent :type Primitive%20Component%20Object%20Reference) (OtherActor :type Actor%20Object%20Reference) (OtherComp :type Primitive%20Component%20Object%20Reference) (NormalImpulse :type Vector :default "0, 0, 0") (Hit :type Hit%20Result%20Structure%20%28by%20ref%29))
  ;[1 1 1] 서브공이 벽돌과 충돌할 때마다 HP가 1씩 깎이며, HP=0일때 소멸
  (Utilities|Casting|CastToB_Brick OtherActor)
  (bind _output_get (Variables|Default|SetSubHP (- (Variables|Default|GetSubHP) 1)))
  (if (<= _output_get 0)
    (Utilities|FlowControl|Delay 0.0) ; 마지막 HP때 벽돌에 데미지를 가하기 위한 방법
    (Actor|DestroyActor)))

(event EventBeginPlay
  ;[1 1 1] 서브공의 HP 및 기본 데미지 세팅
  (|CallParentFunction)
  (Variables|Default|SetSubHP 3)
  (Variables|Default|SetSubDamage 1)
  (CallFunction|SetCausesGameOver false) ; 서브공이 부딪혔을 때는 GameOver가 되지 않음
)

(event Collision|EventActorBeginOverlap
  (params (OtherActor :type Actor%20Object%20Reference)))

(event EventTick
  (params (DeltaSeconds :type Float%20%28single-precision%29))
  ;[1 1 1] 서브공의 위치 업데이트
  (|CallParentFunction DeltaSeconds))

(fn ConstructionScript
  (|CallParentFunction))

(fn SpeedUp)

(fn SpeedDown)

(fn GetDamage
  (return (Variables|Default|GetSubDamage)))

(fn IncreaseDamage)