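; Destructible brick actor for a Breakout game, randomly becoming a tougher red or weaker green brick on BeginPlay.
; Hits from B_Ball subtract the ball's damage from HP and swap the material to show the remaining health.
; At zero HP it destroys itself, notifies GI_BreakOut and plays a break sound.
; GetBrickSize exposes the mesh's full bounds size.
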(event OnComponentHit(SM_Brick)
  (params (HitComponent :type Primitive%20Component%20Object%20Reference) (OtherActor :type Actor%20Object%20Reference) (OtherComp :type Primitive%20Component%20Object%20Reference) (NormalImpulse :type Vector :default "0, 0, 0") (Hit :type Hit%20Result%20Structure%20%28by%20ref%29))
  ;[1 1 1] 공과 충돌했을 때 벽돌의 HP-1
  (bind _asb_ball (Utilities|Casting|CastToB_Ball OtherActor))
  (Utilities|IsValid _asb_ball
    (:Is%20Valid
      (bind _output_get (Variables|Brick|SetCurrentHP (- (Variables|Brick|GetCurrentHP) (Default|GetDamage _asb_ball))))
      (Brick|ChangeColor)
      (if (<= _output_get 0)
        (Utilities|FlowControl|Sequence
          (:then_0
            (Actor|DestroyActor))
          (:then_1
            ;;[1 1 1] 벽돌이 파괴될 때 호출
            (bind _asgi_break_out (Utilities|Casting|CastToGI_BreakOut (Game|GetGameInstance)))
            (Default|OnBrickDestroyed _asgi_break_out)
            (Audio|PlaySound2D "/Game/Sounds/A_BrickBreak.A_BrickBreak" 1.0 1.0 0.0 0 0)))))))

(event EventBeginPlay
  ;[1 1 1] 벽돌 타입 및 HP 세팅
  (Variables|Brick|SetBrickType (Math|Random|RandomIntegerinRange 0 1))
  (Brick|SetBrickType)
  (Variables|Brick|SetCurrentHP (Variables|Brick|GetMaxHP)))

(event Collision|EventActorBeginOverlap
  (params (OtherActor :type Actor%20Object%20Reference)))

(event EventTick
  (params (DeltaSeconds :type Float%20%28single-precision%29)))

(fn ConstructionScript)

(fn SetBrickType
  (switch int (Variables|Brick|GetBrickType)
    (:Default
      (Variables|Brick|SetMaxHP 5 :!label _label) ; 빨간 벽돌
      (Rendering|Material|SetMaterial (Variables|Default|GetSM_Brick) 0 "/Game/3D_Assets/Bricks/MI_Brick_Red_0.MI_Brick_Red_0"))
    (:0
      (goto _label))
    (:1
      (Variables|Brick|SetMaxHP 3) ; 초록 벽돌
      (Rendering|Material|SetMaterial (Variables|Default|GetSM_Brick) 0 "/Game/3D_Assets/Bricks/MI_Brick_Green_0.MI_Brick_Green_0")))
  (return))

(fn ChangeColor
  (bind _sm_brick (Variables|Default|GetSM_Brick))
  (bind _sm_brick_2 (Variables|Default|GetSM_Brick))
  (if (== (Variables|Brick|GetBrickType) 0)
    ;[1 0.159 0.1981] Red Brick
    (switch int (Variables|Brick|GetCurrentHP)
      (:1
        (Rendering|Material|SetMaterial _sm_brick_2 0 "/Game/3D_Assets/Bricks/MI_Brick_Red_4.MI_Brick_Red_4"))
      (:2
        (Rendering|Material|SetMaterial _sm_brick_2 0 "/Game/3D_Assets/Bricks/MI_Brick_Red_3.MI_Brick_Red_3"))
      (:3
        (Rendering|Material|SetMaterial _sm_brick_2 0 "/Game/3D_Assets/Bricks/MI_Brick_Red_2.MI_Brick_Red_2"))
      (:4
        (Rendering|Material|SetMaterial _sm_brick_2 0 "/Game/3D_Assets/Bricks/MI_Brick_Red_1.MI_Brick_Red_1")))
    (else
      ;[0.491 0.9131 0.2195] Green Brick
      (switch int (Variables|Brick|GetCurrentHP)
        (:1
          (Rendering|Material|SetMaterial _sm_brick 0 "/Game/3D_Assets/Bricks/MI_Brick_Green_2.MI_Brick_Green_2"))
        (:2
          (Rendering|Material|SetMaterial _sm_brick 0 "/Game/3D_Assets/Bricks/MI_Brick_Green_1.MI_Brick_Green_1")))))
  (return))

(fn GetBrickSize
  (return (* (.BoxExtent (Collision|GetComponentBounds (Variables|Default|GetSM_Brick))) 2.0)))