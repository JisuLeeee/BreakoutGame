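; B_BrickSpawner builds the breakout brick grid at BeginPlay, laid out around StartLocation on the YZ plane.
; It spawns and immediately destroys a temporary B_Brick to read the brick size, then uses that size plus Spacing as the grid step.
; RowCount runs along Y and ColCount along Z, with index offsets centering the grid.
; It counts valid spawns and passes the total to GI_BreakOut as the alive brick count.
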(event EventBeginPlay
  ;[1 1 1] StartLocaiton 값을 중심으로 대칭적으로 스폰 (행열)
  ;;[1 1 1] 벽돌 사이 간의 간격을 동일하게 유지
  (bind _returnvalue (Game|SpawnActorfromClass "/Game/Blueprints/B_Brick.B_Brick_C" (Math|Transform|MakeTransform "0, 0, 0") "Undefined" "MultiplyWithRoot" 0 0))
  (bind _bricksize (Default|GetBrickSize _returnvalue))
  (Actor|DestroyActor _returnvalue)
  (for _index (range 0 (- (Variables|BrickSpawner|GetRowCount) 1))
    (for _index_2 (range 0 (- (Variables|BrickSpawner|GetColCount) 1))
      (bind _returnvalue_2 (Game|SpawnActorfromClass "/Game/Blueprints/B_Brick.B_Brick_C" (Math|Transform|MakeTransform (+ (Variables|BrickSpawner|GetStartLocation) (Math|Vector|MakeVector 0.0 (* (- _index (/ (- (Variables|BrickSpawner|GetRowCount) 1) 2)) (.y (+ _bricksize (Variables|BrickSpawner|GetSpacing)))) (* (- _index_2 (/ (- (Variables|BrickSpawner|GetColCount) 1) 2)) (.z (+ _bricksize (Variables|BrickSpawner|GetSpacing))))))) "Undefined" "MultiplyWithRoot" 0 0))
      ;[1 1 1] 현재 소환된 벽돌의 갯수 파악
      (Utilities|IsValid _returnvalue_2
        (:Is%20Valid
          (bind _output_get (Variables|BrickSpawner|SetSpawnedCount (+ (Variables|BrickSpawner|GetSpawnedCount) 1))) ; 스폰될때마다 +1을 하기 위해 더함
        ))))
  (bind _asgi_break_out (Utilities|Casting|CastToGI_BreakOut (Game|GetGameInstance)))
  (Default|SetAliveBricks _asgi_break_out _output_get))

(event Collision|EventActorBeginOverlap
  (params (OtherActor :type Actor%20Object%20Reference)))

(event EventTick
  (params (DeltaSeconds :type Float%20%28single-precision%29)))

(fn ConstructionScript)