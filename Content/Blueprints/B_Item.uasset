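; B_Item is a falling pickup for a Breakout game, with an empty ActivateEffect hook for its effect.
; While GI_BreakOut reports the game running and unpaused, Tick sweeps it downward along a direction given a random Y component at spawn.
; Wall hits reflect that direction off the hit normal, and Ground hits destroy the item.
; Overlapping B_Ball or B_Player calls ActivateEffect, destroys it and plays a sound.
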(event OnComponentHit(SM_Item)
  (params (HitComponent :type Primitive%20Component%20Object%20Reference) (OtherActor :type Actor%20Object%20Reference) (OtherComp :type Primitive%20Component%20Object%20Reference) (NormalImpulse :type Vector :default "0, 0, 0") (Hit :type Hit%20Result%20Structure%20%28by%20ref%29))
  (bind _normal (Collision|BreakHitResult Hit))
  ;[1 1 1] 벽에 부딪힐 경우 충돌 상호작용이 발생하며 아이템의 방향이 변함
  (Utilities|FlowControl|Sequence
    (:then_0
      (if (Actor|ActorHasTag OtherActor "Wall")
        (Variables|Item|SetFallDirection (- (Variables|Item|GetFallDirection) (* (* _normal (Math|Vector|DotProduct _normal (Variables|Item|GetFallDirection))) 2.0)))))
    (:then_1
      ;[1 1 1] 바닥에 닿으면 아이템이 사라짐
      (if (Actor|ActorHasTag OtherActor "Ground")
        (Actor|DestroyActor)))))

(event EventBeginPlay
  (bind _asgi_break_out (Utilities|Casting|CastToGI_BreakOut (Game|GetGameInstance)))
  (Variables|Item|SetGI_BreakOut _asgi_break_out)
  ;[1 1 1] Y축기준 랜덤 방향
  (Variables|Item|SetFallDirection (Math|Vector|Normalize (Math|Vector|MakeVector 0.0 (Math|Random|RandomFloatinRange -1.0 1.0) -1.0))))

(event Collision|EventActorBeginOverlap
  (params (OtherActor :type Actor%20Object%20Reference))
  ;[1 1 1] 패들 혹은 공이 아이템과 충돌할 때 발생하는 효과
  (Utilities|Casting|CastToB_Ball OtherActor
    (:then
      (Item|ActivateEffect)
      (Actor|DestroyActor)
      (Audio|PlaySound2D "/Game/Sounds/A_GainItem.A_GainItem" 1.0 1.0 0.0 0 0))
    (:CastFailed
      (Utilities|Casting|CastToB_Player OtherActor)
      (Item|ActivateEffect)
      (Actor|DestroyActor)
      (Audio|PlaySound2D "/Game/Sounds/A_GainItem.A_GainItem" 1.0 1.0 0.0 0 0))))

(event EventTick
  (params (DeltaSeconds :type Float%20%28single-precision%29))
  (bind _gi_breakout (Variables|Item|GetGI_BreakOut))
  ;[1 1 1] 게임이 진행 상태일 때
  (if (and (Default|GetIsRunning _gi_breakout) (not (Default|GetIsPaused _gi_breakout)))
    ;[1 1 1] 아이템의 움직임 (위에서 아래로)
    (Transformation|SetActorLocation (+ (* (* DeltaSeconds (Variables|Item|GetFallSpeed)) (Variables|Item|GetFallDirection)) (Transformation|GetActorLocation)) true false)))

(fn ConstructionScript)

(fn ActivateEffect
  (params (ActorTarget :type Actor%20Object%20Reference))
  (return))