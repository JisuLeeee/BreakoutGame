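; B_ItemSpawner spawns random item actors in the BreakOut game as time, score and combos progress.
; Three looping timers read GI_BreakOut and spawn only while the game runs unpaused.
; Level 1 items follow a time interval; Level 2 and 3 poll for score passing a new bucket or combo count exceeding its last recorded high.
; SpawnRandom picks from that level's class list and randomizes Y/Z position and roll.
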(event EventBeginPlay
  (bind _asgi_break_out (Utilities|Casting|CastToGI_BreakOut (Game|GetGameInstance)))
  (Variables|ItemSpawner|SetLastScoreBucket (/ (Default|GetScore _asgi_break_out) (Variables|ItemSpawner|GetScoreBucketSize)))
  (Variables|ItemSpawner|SetLastComboCount (Default|GetComboCount _asgi_break_out))
  (Utilities|Time|SetTimerbyFunctionName 0 "SpawnLevel1" (Variables|ItemSpawner|GetTimeInterval) true) ; 플레이 타임 10초 경과마다 스폰
  (Utilities|Time|SetTimerbyFunctionName 0 "SpawnLevel2" 0.2 true) ; 스코어가 100점 단위로 쌓일때마다 스폰
  (Utilities|Time|SetTimerbyFunctionName 0 "SpawnLevel3" 0.2 true) ; 콤보가 발동될때마다 스폰
)

(event Collision|EventActorBeginOverlap
  (params (OtherActor :type Actor%20Object%20Reference)))

(fn ConstructionScript)

(fn SpawnRandom
  (params (LevelItem :type Array%20of%20B%20Item%20Class%20References))
  (bind _returnvalue (Utilities|Array|Length LevelItem))
  (if (> _returnvalue 0)
    (Game|SpawnActorfromClass (Utilities|Array|Get(acopy) LevelItem (Math|Random|RandomIntegerinRange 0 (- _returnvalue 1))) (Math|Transform|MakeTransform (+ (Variables|ItemSpawner|GetStartLocation) (Math|Vector|MakeVector 0.0 (Math|Random|RandomFloatinRange -7.2e+02 7.2e+02) (Math|Random|RandomFloatinRange 4e+02 6.4e+02))) (Math|Rotator|MakeRotator (Math|Random|RandomFloatinRange -1.8e+02 1.8e+02) 0.0 0.0)) "Undefined" "MultiplyWithRoot" 0 0)
    (return)))

(fn SpawnLevel1
  (bind _asgi_break_out (Utilities|Casting|CastToGI_BreakOut (Game|GetGameInstance)))
  (if (and (not (Default|GetIsPaused _asgi_break_out)) (Default|GetIsRunning _asgi_break_out))
    (ItemSpawner|SpawnRandom (Variables|ItemSpawner|GetLevel1s))
    (return)))

(fn SpawnLevel2
  (bind _asgi_break_out (Utilities|Casting|CastToGI_BreakOut (Game|GetGameInstance)))
  (if (or (Default|GetIsPaused _asgi_break_out) (not (Default|GetIsRunning _asgi_break_out)))
    (return)
    (elif (> (/ (Default|GetScore _asgi_break_out) (Variables|ItemSpawner|GetScoreBucketSize)) (Variables|ItemSpawner|GetLastScoreBucket))
      (ItemSpawner|SpawnRandom (Variables|ItemSpawner|GetLevel2s))
      (Variables|ItemSpawner|SetLastScoreBucket (/ (Default|GetScore _asgi_break_out) (Variables|ItemSpawner|GetScoreBucketSize))))))

(fn SpawnLevel3
  (bind _asgi_break_out (Utilities|Casting|CastToGI_BreakOut (Game|GetGameInstance)))
  (if (or (Default|GetIsPaused _asgi_break_out) (not (Default|GetIsRunning _asgi_break_out)))
    (return)
    (elif (> (Default|GetComboCount _asgi_break_out) (Variables|ItemSpawner|GetLastComboCount))
      (ItemSpawner|SpawnRandom (Variables|ItemSpawner|GetLevel3s))
      (Variables|ItemSpawner|SetLastComboCount (Default|GetComboCount _asgi_break_out)))))