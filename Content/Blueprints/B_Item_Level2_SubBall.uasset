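; Level 2 sub-ball item that, on activation, replaces existing sub-balls with a fan of new B_BallSub actors around the main ball.
; It first destroys sub-balls owned by MainBallRef, then reads the first B_Ball's position, direction and speed.
; Each SpawnAngles entry rotates the normalized YZ direction about X, setting a sub-ball's heading and clamped-radius offset.
; SetOwner(MainBallRef) targets the item itself, not the spawned sub-balls.
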(event EventBeginPlay)

(event Collision|EventActorBeginOverlap
  (params (OtherActor :type Actor%20Object%20Reference)))

(event EventTick
  (params (DeltaSeconds :type Float%20%28single-precision%29))
  (|CallParentFunction DeltaSeconds) ; This node is disabled and will not be called.\nDrag off pins to build functionality.
)

(fn ConstructionScript
  (|CallParentFunction))

(fn ActivateEffect
  (params (ActorTarget :type Actor%20Object%20Reference))
  (|CallParentFunction ActorTarget)
  ;[1 1 1] 서브공 삭제
  (bind _outactors (Actor|GetAllActorsOfClass "/Game/Blueprints/B_BallSub.B_BallSub_C"))
  (for _array_element _outactors
    (if (== (Components|GetOwner _array_element) (Variables|Level2_SubBall|GetMainBallRef))
      (Actor|DestroyActor _array_element)))
  (bind _outactors_2 (Actor|GetAllActorsOfClass "/Game/Blueprints/B_Ball.B_Ball_C"))
  ;[1 1 1] 서브공 방향 (BaseDirection에서 Spawn Angle 만큼 X축으로 회전)
  (for _array_element_2 (Variables|Level2_SubBall|GetSpawnAngles)
    (bind _returnvalue (Game|SpawnActorfromClass "/Game/Blueprints/B_BallSub.B_BallSub_C" (Math|Transform|MakeTransform (+ (* (Math|Vector|RotateVectorAroundAxis (Math|Vector|Normalize (Math|Vector|MakeVector 0.0 (.Y (Math|Vector|BreakVector (Default|GetDirection (Utilities|Array|Get(acopy) _outactors_2)))) (.Z (Math|Vector|BreakVector (Default|GetDirection (Utilities|Array|Get(acopy) _outactors_2)))))) _array_element_2 "1.000000,0.000000,0.000000") (Math|Integer|Clamp(Integer) (Variables|Level2_SubBall|GetSpawnRadius) 0 30)) (Default|GetLocation (Utilities|Array|Get(acopy) _outactors_2)))) "Undefined" "MultiplyWithRoot" 0 0))
    (Default|SetDirection _returnvalue (Math|Vector|RotateVectorAroundAxis (Math|Vector|Normalize (Math|Vector|MakeVector 0.0 (.Y (Math|Vector|BreakVector (Default|GetDirection (Utilities|Array|Get(acopy) _outactors_2)))) (.Z (Math|Vector|BreakVector (Default|GetDirection (Utilities|Array|Get(acopy) _outactors_2)))))) _array_element_2 "1.000000,0.000000,0.000000"))
    (Default|SetSpeed _returnvalue (Default|GetSpeed (Utilities|Array|Get(acopy) _outactors_2)))
    (Actor|SetOwner (Variables|Level2_SubBall|GetMainBallRef)))
  (return))