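; B_Player is the player-controlled paddle of a Breakout game, with timed enlarge and sub-ball shooting effects.
; Enhanced Input slides the paddle along Y only while GI_BreakOut reports running and unpaused, with tighter clamps when enlarged.
; InrcreasePaddleSize widens the paddle and starts a reset timer, restarting it on repeat calls instead of stacking scale.
; ShotSubBall loops a timer spawning upward-moving B_BallSub actors until a second timer stops it.
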(event Input|EnhancedActionEvents|EnhancedInputActionIA_Move
  (params (ActionValue :type Float%20%28double-precision%29) (ElapsedSeconds :type Float%20%28double-precision%29) (TriggeredSeconds :type Float%20%28double-precision%29) (InputAction :type Input%20Action%20Object%20Reference :default "/Game/Input/IA_Move.IA_Move"))
  (bind _sm_paddle (Variables|Default|GetSM_Paddle))
  (bind _paddlespeed (Variables|Player|GetPaddleSpeed))
  (bind _gi_breakout (Variables|Player|GetGI_BreakOut))
  (bind _returnvalue (* ActionValue _paddlespeed))
  (bind _relativelocation (Variables|/Script/Engine.SceneComponent|GetRelativeLocation _sm_paddle))
  (bind (_x _y _z) (Math|Vector|BreakVector _relativelocation))
  (bind _returnvalue_2 (+ _returnvalue _y))
  ;[1 1 1] 게임이 진행 상태일 때
  (if (and (Default|GetIsRunning _gi_breakout) (not (Default|GetIsPaused _gi_breakout)))
    ;[1 1 1] Y축 방향을 기준으로 움직임
    (if (Variables|Player|GetbIsPaddleEnlarged)
      ;;[1 1 1] Paddle의 사이즈가 커졌을 때 Paddle이 움직이는 범위
      (Transformation|SetRelativeLocation (Variables|Default|GetSM_Paddle) (Math|Vector|MakeVector _x (Math|Float|Clamp(Float) _returnvalue_2 -4.5e+02 4.5e+02) _z) false false)
      (else
        ;;[1 1 1] Paddle의 사이즈가 커지지 않았을 때 Paddle이 움직이는 범위
        (Transformation|SetRelativeLocation (Variables|Default|GetSM_Paddle) (Math|Vector|MakeVector _x (Math|Float|Clamp(Float) _returnvalue_2 -6e+02 6e+02) _z) false false)))))

(event EventBeginPlay
  (bind _asgi_break_out (Utilities|Casting|CastToGI_BreakOut (Game|GetGameInstance)))
  (Variables|Player|SetGI_BreakOut _asgi_break_out)
  ;[1 1 1] Input Mapping 세팅
  (bind _asplayer_controller (Utilities|Casting|CastToPlayerController (Pawn|GetController)))
  (Utilities|IsValid (PlayerController|LocalPlayerSubsystems|GetEnhancedInputLocalPlayerSubsystem _asplayer_controller)
    (:Is%20Valid
      (Input|AddMappingContext (PlayerController|LocalPlayerSubsystems|GetEnhancedInputLocalPlayerSubsystem _asplayer_controller) "/Game/Input/IMC_Player.IMC_Player" 0 "(bIgnoreAllPressedKeysUntilRelease=True,bForceImmediately=False,bNotifyUserSettings=False)"))))

(fn ConstructionScript)

(fn InrcreasePaddleSize
  (if (Variables|Player|GetbIsPaddleEnlarged)
    ;[1 1 1] Paddle 사이즈가 커지면 6초 후에 크기 리셋
    (Utilities|Time|SetTimerbyFunctionName 0 "ResetPaddleSize" 6.0)
    (else
      ;[1 1 1] Paddle 사이즈가 커지지 않았다면 Y방향으로 3만큼 크기 증가
      (bind _output_get (Variables|Player|SetPaddleSize (Variables|/Script/Engine.SceneComponent|GetRelativeScale3D (Variables|Default|GetSM_Paddle))))
      (Transformation|SetRelativeScale3D (Variables|Default|GetSM_Paddle) (Math|Vector|MakeVector (.X (Math|Vector|BreakVector _output_get)) (+ (.Y (Math|Vector|BreakVector _output_get)) 3.0) (.Z (Math|Vector|BreakVector _output_get))))
      (Variables|Player|SetbIsPaddleEnlarged true)
      (Utilities|Time|SetTimerbyFunctionName 0 "ResetPaddleSize" 6.0)))
  (return))

(fn ResetPaddleSize
  (Transformation|SetRelativeScale3D (Variables|Default|GetSM_Paddle) (Variables|Player|GetPaddleSize))
  (Variables|Player|SetbIsPaddleEnlarged false)
  (return))

(fn ShotSubBall
  (bind _returnvalue (Utilities|Time|SetTimerbyFunctionName 0 "ShotOnce" (Variables|Player|GetShotInterval) true))
  (Variables|Player|SetHandleShot _returnvalue) ; 타이머를 중지(ClearTimer)
  (bind _returnvalue_2 (Utilities|Time|SetTimerbyFunctionName 0 "StopEffect" (Variables|Player|GetEffectDuration)))
  (Variables|Player|SetHandleStop _returnvalue_2)
  (return))

(fn ShotOnce
  (bind _returnvalue (Game|SpawnActorfromClass "/Game/Blueprints/B_BallSub.B_BallSub_C" (Math|Transform|MakeTransform (+ (Transformation|GetWorldLocation (Variables|Default|GetSM_Paddle)) "0.000000,0.000000,50.000000")) "Undefined" "MultiplyWithRoot" 0 0))
  (Default|SetDirection _returnvalue (Math|Vector|MakeVector 0.0 0.0 1.0))
  (Default|SetSpeed _returnvalue (Variables|Player|GetShotSpeed))
  (return))

(fn StopEffect
  (Utilities|Time|ClearandInvalidateTimerbyHandle (Variables|Player|GetHandleShot))
  (Utilities|Time|ClearandInvalidateTimerbyHandle (Variables|Player|GetHandleStop))
  (return))