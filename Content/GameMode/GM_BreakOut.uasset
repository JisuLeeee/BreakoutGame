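; GM_BreakOut is the game mode for a Breakout game, handling startup UI and driving the round timer.
; On BeginPlay it sets windowed mode, shows the mouse cursor and caches the GI_BreakOut game instance.
; A game-instance flag, cleared once read, chooses between the countdown widget and the start menu on level open.
; Tick forwards delta time to the game instance's TickRound while the round is running and unpaused.
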(event EventBeginPlay
  (Utilities|FlowControl|Sequence
    (:then_0
      (bind _returnvalue (Settings|GetGameUserSettings))
      (Class|GameUserSettings|SetFullscreenMode _returnvalue "Windowed")
      (Class|GameUserSettings|ApplyResolutionSettings _returnvalue false)
      (Variables|/Script/Engine.PlayerController|SetbShowMouseCursor (Game|GetPlayerController 0) true))
    (:then_1
      (bind _asgi_break_out (Utilities|Casting|CastToGI_BreakOut (Game|GetGameInstance)))
      (Variables|GM_Breakout|SetGI_Breakout _asgi_break_out))
    (:then_2
      ;[1 1 1] StartatCountCountdown 상태에 따라, OpenLevel시 처음 시작되는 위젯 세팅
      (if (Default|GetStartatCountdown (Variables|GM_Breakout|GetGI_Breakout))
        (Default|SetStartatCountdown (Variables|GM_Breakout|GetGI_Breakout) false)
        (bind _returnvalue_2 (UserInterface|CreateWidget "/Game/UserInterface/W_Countdown.W_Countdown_C"))
        (bind _output_get (Variables|GM_Breakout|SetCountdown%20Widget _returnvalue_2))
        (UserInterface|Viewport|AddtoViewport _output_get 0)
        (Widget|SetVisibility (Variables|GM_Breakout|GetCountdown%20Widget) "Visible")
        (else
          (bind _returnvalue_3 (UserInterface|CreateWidget "/Game/UserInterface/W_StartMenu.W_StartMenu_C"))
          (bind _output_get_2 (Variables|GM_Breakout|SetStartgame%20Widget _returnvalue_3))
          (UserInterface|Viewport|AddtoViewport _output_get_2 0)
          (Widget|SetVisibility (Variables|GM_Breakout|GetStartgame%20Widget) "Visible"))))))

(event EventTick
  (params (DeltaSeconds :type Float%20%28single-precision%29))
  ;[1 1 1] Running=True, Paused=False일 때, TickRound(경과시간 및 제한시간) 실행
  (if (and (Default|GetIsRunning (Variables|GM_Breakout|GetGI_Breakout)) (not (Default|GetIsPaused (Variables|GM_Breakout|GetGI_Breakout))))
    (Default|TickRound (Variables|GM_Breakout|GetGI_Breakout) DeltaSeconds) ; 경과시간 및 제한시간 실행, 패배조건 감지(제한시간 넘었을 때)
  ))

(fn ConstructionScript)